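; LevelDesignArea_BP is a level area actor that serves as a camera view target, with a test of a Celeste-style camera.
; On BeginPlay it takes the player's view if flagged as first, and either picks a random background mesh or, rarely, hides the background.
; With ShouldFollowPlayer set, it always hides the background and matches the player capsule's height each Tick, keeping its own X and Y.
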(event `self.ReceiveBeginPlay`
  (set `self.Backgrounds` (`|MakeArray` "/Game/importMesh/Decor/backgroundWall/1.1" "/Game/importMesh/Decor/backgroundWall/2.2" "/Game/importMesh/Decor/backgroundWall/3.3" "/Game/importMesh/Decor/backgroundWall/4.4" "/Game/importMesh/Decor/backgroundWall/5.5" :!type "StaticMesh Object Reference"))
  ;[1 1 1] Test Camera Celeste
  (if (`self.shouldFollowPlayer`)
    (`SceneComponent.SetVisibility` (`self.background`) false false :!label _label)
    (elif (> (`KismetMathLibrary.RandomFloat`) 0.01)
      (`StaticMeshComponent.SetStaticMesh` (`self.background`) (`KismetArrayLibrary.Array_Random` (`self.Backgrounds`)))
      (else
        (goto _label))))
  (if (`self.isFirst`)
    (`PlayerController.SetViewTargetWithBlend` (`GameplayStatics.GetPlayerController` 0) self 0.0 "VTBlend_Linear" 0.0 false)))

(event `self.ReceiveTick`
  (params (DeltaSeconds :type "Float (single-precision)"))
  (bind (_returnvalue_x _returnvalue_y) (`KismetMathLibrary.BreakVector` (`self.K2_GetActorLocation` self)))
  (bind (_returnvalue_x_2 _returnvalue_y_2 _returnvalue_z) (`KismetMathLibrary.BreakVector` (`SceneComponent.K2_GetComponentLocation` (`Character.CapsuleComponent` (`GameplayStatics.GetPlayerCharacter` 0)))))
  (if (`self.shouldFollowPlayer`)
    (`self.K2_SetActorLocation` (`KismetMathLibrary.MakeVector` _returnvalue_x _returnvalue_y _returnvalue_z))))

(fn `UserConstructionScript`)