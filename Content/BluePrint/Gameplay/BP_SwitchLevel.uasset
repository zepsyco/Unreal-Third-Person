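; BP_SwitchLevel is a trigger that switches the camera and updates the respawn point when the player enters its box.
; On overlap by player character 0, it blends the view to CamRef over a short time.
; It then finds RespawnPosSave among all BP_SpawnPos actors and stores its array index in BP_ThirdPersonCharacter's RespawnPos, so the saved value depends on GetAllActorsOfClass ordering.
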(event `self.Box.OnComponentBeginOverlap`
  (params (OverlappedComponent :type "PrimitiveComponent Object Reference") (OtherActor :type "Actor Object Reference") (OtherComp :type "PrimitiveComponent Object Reference") (OtherBodyIndex :type Integer) (bFromSweep :type Boolean) (SweepResult :type "HitResult Structure (by ref)"))
  (bind _returnvalue (`GameplayStatics.GetPlayerCharacter` 0))
  (if (== OtherActor _returnvalue)
    (`PlayerController.SetViewTargetWithBlend` (`GameplayStatics.GetPlayerController` 0) (`self.camRef`) 1.0 "VTBlend_Linear" 0.0 false)
    (bind _outactors (`GameplayStatics.GetAllActorsOfClass` "/Game/BluePrint/Gameplay/BP_SpawnPos.BP_SpawnPos_C"))
    (for (_array_element _array_index) _outactors
      (if (== _array_element (`self.respawnPosSave`))
        (bind _asbp_third_person_character (cast `/Game/ThirdPerson/Blueprints/BP_ThirdPersonCharacter` _returnvalue))
        (set `/Game/ThirdPerson/Blueprints/BP_ThirdPersonCharacter.respawnPos` _array_index _asbp_third_person_character)))))

(fn `UserConstructionScript`)