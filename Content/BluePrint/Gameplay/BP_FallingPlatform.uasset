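; BP_FallingPlatform is a platform that shakes, drops and respawns after the player character overlaps its Box trigger.
; The overlap handler sequences the phases with delays and the IsShaking and IsFalling flags.
; Shake and Fall are self-calling delayed events that move the Cube by random offsets or steady downward steps, without physics simulation.
; The Cube is then hidden, reset to its relative origin and shown again after a short delay.
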(event `respawnPlatform`
  (bind _cube (`self.Cube`))
  (`PrimitiveComponent.SetSimulatePhysics` _cube false)
  (`SceneComponent.K2_SetRelativeLocation` _cube (0.0 0.0 0.0) false false)
  (`KismetSystemLibrary.Delay` 0.2)
  (`SceneComponent.SetVisibility` _cube true false))

(event `Fall`
  (bind (_relativelocation_x _relativelocation_y _relativelocation_z) (`KismetMathLibrary.BreakVector` (`SceneComponent.RelativeLocation` (`self.Cube`))))
  (if (`self.isFalling`)
    (`SceneComponent.K2_SetRelativeLocation` (`self.Cube`) (`KismetMathLibrary.MakeVector` _relativelocation_x _relativelocation_y (- _relativelocation_z 10.0)) false false)
    (`KismetSystemLibrary.Delay` 0.01)
    (`self.Fall`)))

(event `Shake`
  (if (`self.isFalling`)
    _
    (elif (`self.isShaking`)
      (`SceneComponent.K2_SetRelativeLocation` (`self.Cube`) (* (`KismetMathLibrary.RandomUnitVector`) 10.0) false false)
      (`KismetSystemLibrary.Delay` 0.01)
      (`self.Shake`))))

(event `self.Box.OnComponentBeginOverlap`
  (params (OverlappedComponent :type "PrimitiveComponent Object Reference") (OtherActor :type "Actor Object Reference") (OtherComp :type "PrimitiveComponent Object Reference") (OtherBodyIndex :type Integer) (bFromSweep :type Boolean) (SweepResult :type "HitResult Structure (by ref)"))
  (if (== OtherActor (`GameplayStatics.GetPlayerCharacter` 0))
    (set `self.isShaking` true)
    (`self.Shake`)
    (`KismetSystemLibrary.Delay` 1.0)
    (set `self.isShaking` false)
    (set `self.isFalling` true)
    (`self.Fall`)
    (`KismetSystemLibrary.Delay` 2.0)
    (`SceneComponent.SetVisibility` (`self.Cube`) false false)
    (set `self.isFalling` false)
    (`self.respawnPlatform`)))

(fn `UserConstructionScript`)