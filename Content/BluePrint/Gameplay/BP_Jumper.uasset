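; BP_Jumper is a jump pad that launches the player high into the air when they enter its box trigger.
; The overlap temporarily raises the third-person character's jump velocity and simulates a jump, then sets the velocity back to a hardcoded value.
; Meanwhile recursive, Delay-stepped events raise the Cube2 plate, pause, lower it, then clear the flags that block retriggering.
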(event `pushPlayer`
  (set `self.playerPushed` true)
  (bind _asbp_third_person_character (cast `/Game/ThirdPerson/Blueprints/BP_ThirdPersonCharacter` (`GameplayStatics.GetPlayerCharacter` 0)))
  (bind _charactermovement (`Character.CharacterMovement` _asbp_third_person_character))
  (set `CharacterMovementComponent.JumpZVelocity` 2500.0 _charactermovement)
  (`/Game/ThirdPerson/Blueprints/BP_ThirdPersonCharacter.simulateJump` _asbp_third_person_character)
  (`KismetSystemLibrary.Delay` 0.2)
  (set `CharacterMovementComponent.JumpZVelocity` 1500.0 _charactermovement))

(event `pushJumper`
  (bind _cube2 (`self.Cube2`))
  (bind (_relativelocation_x _relativelocation_y _relativelocation_z) (`KismetMathLibrary.BreakVector` (`SceneComponent.RelativeLocation` _cube2)))
  (bind (_relativelocation_x_2 _relativelocation_y_2 _relativelocation_z_2) (`KismetMathLibrary.BreakVector` (`SceneComponent.RelativeLocation` _cube2)))
  (if (not (`self.playerPushed`))
    (`self.pushPlayer`))
  (if (< _relativelocation_z -50.0)
    (`SceneComponent.K2_SetRelativeLocation` _cube2 (`KismetMathLibrary.MakeVector` _relativelocation_x_2 _relativelocation_y_2 (+ _relativelocation_z_2 10.0)) false false)
    (`KismetSystemLibrary.Delay` 0.01)
    (`self.pushJumper`)
    (else
      (`KismetSystemLibrary.Delay` 0.5)
      (`self.retractJumper`))))

(event `retractJumper`
  (bind _cube2 (`self.Cube2`))
  (bind (_relativelocation_x _relativelocation_y _relativelocation_z) (`KismetMathLibrary.BreakVector` (`SceneComponent.RelativeLocation` _cube2)))
  (bind (_relativelocation_x_2 _relativelocation_y_2 _relativelocation_z_2) (`KismetMathLibrary.BreakVector` (`SceneComponent.RelativeLocation` _cube2)))
  (if (> _relativelocation_z -100.0)
    (`SceneComponent.K2_SetRelativeLocation` _cube2 (`KismetMathLibrary.MakeVector` _relativelocation_x_2 _relativelocation_y_2 (- _relativelocation_z_2 10.0)) false false)
    (`KismetSystemLibrary.Delay` 0.01)
    (`self.retractJumper`)
    (else
      (`KismetSystemLibrary.Delay` 0.2)
      (bind _output_get (set `self.pushed` false))
      (set `self.playerPushed` _output_get))))

(event `self.Box.OnComponentBeginOverlap`
  (params (OverlappedComponent :type "PrimitiveComponent Object Reference") (OtherActor :type "Actor Object Reference") (OtherComp :type "PrimitiveComponent Object Reference") (OtherBodyIndex :type Integer) (bFromSweep :type Boolean) (SweepResult :type "HitResult Structure (by ref)"))
  (if (== OtherActor (`GameplayStatics.GetPlayerCharacter` 0))
    (if (not (`self.pushed`))
      (`self.pushJumper`)
      (set `self.pushed` true))))

(fn `UserConstructionScript`)