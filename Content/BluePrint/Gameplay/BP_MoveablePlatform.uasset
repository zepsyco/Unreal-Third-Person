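; BP_MoveablePlatform is a platform that travels to an end position after the player enters its trigger box, then returns to its start.
; After a short delay, it steps BP1's relative location by a fraction of EndPos through self-recalling events with tiny delays instead of Tick.
; Within a tolerance of the end, it pauses and resets in smaller, slower steps, with IsInReset blocking forward movement until done.
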(event `self.Box.OnComponentBeginOverlap`
  (params (OverlappedComponent :type "PrimitiveComponent Object Reference") (OtherActor :type "Actor Object Reference") (OtherComp :type "PrimitiveComponent Object Reference") (OtherBodyIndex :type Integer) (bFromSweep :type Boolean) (SweepResult :type "HitResult Structure (by ref)"))
  (if (== OtherActor (`GameplayStatics.GetPlayerCharacter` 0))
    (`KismetSystemLibrary.Delay` 0.5)
    (`self.movePlatform`)))

(event `movePlatform`
  (bind _bp_1 (`self.BP_1`))
  (bind _relativelocation (`SceneComponent.RelativeLocation` (`self.endPos`)))
  (bind _relativelocation_2 (`SceneComponent.RelativeLocation` _bp_1))
  (if (`self.isInReset`)
    _
    (elif (!= _relativelocation_2 _relativelocation :`ErrorTolerance` 75.0)
      (`SceneComponent.K2_SetRelativeLocation` _bp_1 (+ _relativelocation_2 (/ _relativelocation (20.0 20.0 20.0))) false false)
      (`KismetSystemLibrary.Delay` 0.01)
      (`self.movePlatform`)
      (else
        (`KismetSystemLibrary.Delay` 0.5)
        (`self.resetPlatform`)))))

(event `resetPlatform`
  (bind _bp_1 (`self.BP_1`))
  (bind _relativelocation (`SceneComponent.RelativeLocation` _bp_1))
  (set `self.isInReset` true)
  (if (!= _relativelocation (`SceneComponent.RelativeLocation` (`self.startPos`)) :`ErrorTolerance` 50.0)
    (`SceneComponent.K2_SetRelativeLocation` _bp_1 (- _relativelocation (/ (`SceneComponent.RelativeLocation` (`self.endPos`)) 50.0)) false false)
    (`KismetSystemLibrary.Delay` 0.01)
    (`self.resetPlatform`)
    (else
      (set `self.isInReset` false))))

(fn `UserConstructionScript`)